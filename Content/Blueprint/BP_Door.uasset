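; BP_Door is an interactable door that moves the player to another level.
; On Interact it runs OpenDoor, which does nothing if the door is locked.
; Otherwise it stores the next level value in GI_YolkoGameInstance, plays a door sound that persists across the transition, and opens the next level by name.
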(event `/Game/Blueprint/Interface/BPI_Interact.Interact`
  (`self.OpenDoor`))

(event `OpenDoor`
  (if (not (`self.isLocked`))
    (bind _asgi_yolko_game_instance (cast `/Game/Blueprint/GameInstance/GI_YolkoGameInstance` (`GameplayStatics.GetGameInstance`)))
    (set `/Game/Blueprint/GameInstance/GI_YolkoGameInstance.CurrentLevel` (`self.NextLevelValue`) _asgi_yolko_game_instance)
    (`GameplayStatics.SpawnSound2D` "/Game/Audio/Door_FIXED.Door_FIXED" 1.0 1.0 0.0 null true)
    (`GameplayStatics.OpenLevel` (`self.NextLevelName`))))

(fn `UserConstructionScript`)