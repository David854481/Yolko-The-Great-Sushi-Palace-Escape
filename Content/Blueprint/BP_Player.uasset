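; Player character for Yolko: an animated sprite moved on the X/Y plane with Enhanced Input.
; Movement plays the flipbook and mirrors it by negative X scale on pure Y input, rewinding when released.
; Capsule overlaps send InteractMessage to the other actor, and Pause opens a cached WB_Pause menu.
; Restart and Hint read CurrentLevel from the game instance to reload the room or play its hint cutscene, varying by InsideOtherRoom in the third.
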(event `self.ReceiveBeginPlay`
  ;[1 1 1] Enables Enhanced Input Local Player Subsystem
  (`PaperFlipbookComponent.Stop` (`self.Sprite`))
  (bind _asplayer_controller (cast `PlayerController` (`self.GetController`)))
  (bind _returnvalue (pcsubsystem `EnhancedInputLocalPlayerSubsystem` _asplayer_controller))
  (`/Engine/EditorBlueprintResources/StandardMacros.IsValid` _returnvalue
    (:`Is Valid`
      (`EnhancedInputSubsystemInterface.AddMappingContext` _returnvalue "/Game/Input/Yolko_IMC.Yolko_IMC" 0 (struct))
      (bind _asgi_yolko_game_instance (cast `/Game/Blueprint/GameInstance/GI_YolkoGameInstance` (`GameplayStatics.GetGameInstance`)))
      (set `self.yolkoGameInstance` _asgi_yolko_game_instance))))

(event `EnhancedInput|/Game/Input/Move_IA`
  (params (ActionValue :type "Vector2D Structure") (ElapsedSeconds :type "Float (double-precision)") (TriggeredSeconds :type "Float (double-precision)") (InputAction :type "InputAction Object Reference" :default "/Game/Input/Move_IA.Move_IA"))
  (bind _sprite (`self.Sprite`))
  (bind _sprite_2 (`self.Sprite`))
  ;[1 1 1] Move_IA Movement
  (:`Triggered`
    (`PaperFlipbookComponent.Play` _sprite)
    (`self.AddMovementInput` (1.0 0.0 0.0) ActionValue_X)
    (`self.AddMovementInput` (0.0 1.0 0.0) ActionValue_Y)
    (if (!= ActionValue_X 0.0)
      _
      (elif (>= ActionValue_Y 0.0)
        (`SceneComponent.SetWorldScale3D` _sprite_2 (-0.25 0.25 0.25)) ; Face Right
        (else
          (`SceneComponent.SetWorldScale3D` _sprite_2 (0.25 0.25 0.25)) ; Face Left
        ))))
  (:`Completed`
    (`PaperFlipbookComponent.Stop` _sprite)
    (`PaperFlipbookComponent.SetPlaybackPosition` _sprite 0.0 false)))

(event `self.CapsuleComponent.OnComponentBeginOverlap`
  (params (OverlappedComponent :type "PrimitiveComponent Object Reference") (OtherActor :type "Actor Object Reference") (OtherComp :type "PrimitiveComponent Object Reference") (OtherBodyIndex :type Integer) (bFromSweep :type Boolean) (SweepResult :type "HitResult Structure (by ref)"))
  ;[1 1 1] Interface
  (message `/Game/Blueprint/Interface/BPI_Interact.Interact` OtherActor))

(event `EnhancedInput|/Game/Input/Pause_IA`
  (params (ActionValue :type Boolean) (ElapsedSeconds :type "Float (double-precision)") (TriggeredSeconds :type "Float (double-precision)") (InputAction :type "InputAction Object Reference" :default "/Game/Input/Pause_IA.Pause_IA"))
  (bind _returnvalue (`GameplayStatics.GetPlayerController` 0))
  (bind _pause_menu_reference (`self.Pause Menu Reference`))
  ;[1 1 1] Pause
  (:`Started`
    (`/Engine/EditorBlueprintResources/StandardMacros.IsValid` (`self.Pause Menu Reference`)
      (:`Is Valid`
        _)
      (:`Is Not Valid`
        (bind _returnvalue_2 (`|CreateWidget` "/Game/UI/WB_Pause.WB_Pause_C"))
        (set `self.Pause Menu Reference` _returnvalue_2)))
    (set `PlayerController.bShowMouseCursor` true _returnvalue)
    (`WidgetBlueprintLibrary.SetInputMode_UIOnlyEx` _returnvalue _pause_menu_reference)
    (`UserWidget.AddToViewport` _pause_menu_reference 0)
    (`GameplayStatics.SetGamePaused` true)))

(event `EnhancedInput|/Game/Input/Restart_IA`
  (params (ActionValue :type Boolean) (ElapsedSeconds :type "Float (double-precision)") (TriggeredSeconds :type "Float (double-precision)") (InputAction :type "InputAction Object Reference" :default "/Game/Input/Restart_IA.Restart_IA"))
  ;[1 1 1] Restart
  (:`Started`
    (if (not (`GameplayStatics.IsGamePaused`))
      (switch `int` (`/Game/Blueprint/GameInstance/GI_YolkoGameInstance.CurrentLevel` (`self.yolkoGameInstance`))
        (:`Default`
          (`GameplayStatics.OpenLevel` "Room1" :!label _label))
        (:`0`
          (goto _label))
        (:`1`
          (`GameplayStatics.OpenLevel` "Room2"))
        (:`2`
          (`GameplayStatics.OpenLevel` "Room3"))))))

(event `EnhancedInput|/Game/Input/Hint_IA`
  (params (ActionValue :type Boolean) (ElapsedSeconds :type "Float (double-precision)") (TriggeredSeconds :type "Float (double-precision)") (InputAction :type "InputAction Object Reference" :default "/Game/Input/Hint_IA.Hint_IA"))
  (bind _yolkogameinstance (`self.yolkoGameInstance`))
  (:`Started`
    (if (not (`GameplayStatics.IsGamePaused`))
      (switch `int` (`/Game/Blueprint/GameInstance/GI_YolkoGameInstance.CurrentLevel` (`self.yolkoGameInstance`))
        (:`0`
          (`/Game/Blueprint/GameInstance/GI_YolkoGameInstance.PlayCutsceneHint` _yolkogameinstance 1 16))
        (:`1`
          (`/Game/Blueprint/GameInstance/GI_YolkoGameInstance.PlayCutsceneHint` _yolkogameinstance 5 33))
        (:`2`
          (if (`self.insideOtherRoom`)
            (`/Game/Blueprint/GameInstance/GI_YolkoGameInstance.PlayCutsceneHint` _yolkogameinstance 4 72)
            (else
              (`/Game/Blueprint/GameInstance/GI_YolkoGameInstance.PlayCutsceneHint` _yolkogameinstance 4 56))))))))

(fn `Interact`)

(fn `SetHintVariables`
  (params (NewParam :type Integer) (NewParam1 :type Integer) (NewParam2 :type Integer)))

(fn `UserConstructionScript`)