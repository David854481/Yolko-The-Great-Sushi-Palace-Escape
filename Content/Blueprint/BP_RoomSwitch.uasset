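; BP_RoomSwitch is an interactable that moves the player between rooms.
; Interact calls ChangeLocation, which teleports the BP_Player character to a configured spawn transform and sets its camera to a configured relative position.
; It also copies the PlayerIsInOtherRoom setting into the player's InsideOtherRoom flag, recording which side of the switch the player is on.
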(event `/Game/Blueprint/Interface/BPI_Interact.Interact`
  (`self.Change Location`))

(event `Change Location`
  (bind _asbp_player (cast `/Game/Blueprint/BP_Player` (`GameplayStatics.GetPlayerCharacter` 0)))
  (`SceneComponent.K2_SetRelativeLocation` (`/Game/Blueprint/BP_Player.Camera` _asbp_player) (`self.NewCameraPosition`) false true)
  (`self.K2_SetActorTransform` _asbp_player (`self.PlayerSpawnPosition`) false true)
  (if (`self.PlayerIsInOtherRoom`)
    (set `/Game/Blueprint/BP_Player.insideOtherRoom` true _asbp_player)
    (else
      (set `/Game/Blueprint/BP_Player.insideOtherRoom` false _asbp_player))))

(fn `UserConstructionScript`)