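; BP_Key is an interactable key pickup that unlocks the level's door.
; On BeginPlay it picks one of three key sprites based on the game instance's current level.
; Interacting unlocks the first BP_Door found, shows the key icon on the HUD widget held by the game mode, plays a pickup sound and destroys the key.
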(event `/Game/Blueprint/Interface/BPI_Interact.Interact`
  (`self.PickupKey`))

(event `PickupKey`
  (bind _returnvalue (`GameplayStatics.GetActorOfClass` "/Game/Blueprint/BP_Door.BP_Door_C"))
  (set `/Game/Blueprint/BP_Door.isLocked` false _returnvalue)
  (bind _asyolko_game_mode_base (cast `/Game/Blueprint/YolkoGameModeBase` (`GameplayStatics.GetGameMode`)))
  (set `Widget.Visibility` "Visible" (`/Game/UI/WB_GameUI.KeyImage` (`/Game/Blueprint/YolkoGameModeBase.WidgetReference` _asyolko_game_mode_base)))
  (`GameplayStatics.PlaySound2D` "/Game/Audio/Pocket_Keys_FIXED.Pocket_Keys_FIXED" 1.0 1.0 0.0 null null)
  (`self.K2_DestroyActor`))

(event `self.ReceiveBeginPlay`
  (bind _keysprite (`self.KeySprite`))
  (bind _asgi_yolko_game_instance (cast `/Game/Blueprint/GameInstance/GI_YolkoGameInstance` (`GameplayStatics.GetGameInstance`)))
  (switch `int` (`/Game/Blueprint/GameInstance/GI_YolkoGameInstance.CurrentLevel` _asgi_yolko_game_instance)
    (:`0`
      (`PaperSpriteComponent.SetSprite` _keysprite "/Game/Sprites/UI/KeyHUD_yolkowabi_1_Sprite.KeyHUD_yolkowabi_1_Sprite"))
    (:`1`
      (`PaperSpriteComponent.SetSprite` _keysprite "/Game/Sprites/UI/KeyHUD_kaniroll_1_Sprite.KeyHUD_kaniroll_1_Sprite"))
    (:`2`
      (`PaperSpriteComponent.SetSprite` _keysprite "/Game/Sprites/UI/KeyHUD_unnieunaggie_1_Sprite.KeyHUD_unnieunaggie_1_Sprite"))))

(fn `UserConstructionScript`)