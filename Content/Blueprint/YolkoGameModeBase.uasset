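; Game mode for Yolko that shows the game UI at start and spawns a key once two sets of unlock triggers are satisfied.
; Events add to or remove from two clamped counters, commented as the Unaggie and Unnie unlock triggers.
; When KeyCanSpawn is set, each increment checks both counters against their maximums and, through a DoOnce, spawns BP_Key at a stored transform.
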(event `AddTrigger2UnlockAmount`
  ;[1 1 1] Unnie Unlock Trigger
  (set `self.Trigger2_UnlockTriggerAmount` (`KismetMathLibrary.Clamp` (+ (`self.Trigger2_UnlockTriggerAmount`) 1) 0 (`self.Trigger2_MaxTriggerAmount`)))
  (if (`self.KeyCanSpawn`)
    (`self.CheckIfDoorUnlockable`)))

(event `RemoveTrigger2UnlockAmount`
  ;[1 1 1] Unnie Unlock Trigger
  (set `self.Trigger2_UnlockTriggerAmount` (`KismetMathLibrary.Clamp` (- (`self.Trigger2_UnlockTriggerAmount`) 1) 0 (`self.Trigger2_MaxTriggerAmount`))))

(event `AddTrigger1UnlockAmount`
  ;[1 1 1] Unaggie Unlock Trigger
  (set `self.Trigger1_UnlockTriggerAmount` (`KismetMathLibrary.Clamp` (+ (`self.Trigger1_UnlockTriggerAmount`) 1) 0 (`self.Trigger1_MaxTriggerAmount`)))
  (if (`self.KeyCanSpawn`)
    (`self.CheckIfDoorUnlockable`)))

(event `RemoveTrigger1TriggerAmount`
  ;[1 1 1] Unaggie Unlock Trigger
  (set `self.Trigger1_UnlockTriggerAmount` (`KismetMathLibrary.Clamp` (- (`self.Trigger1_UnlockTriggerAmount`) 1) 0 (`self.Trigger1_MaxTriggerAmount`))))

(event `CheckIfDoorUnlockable`
  ;[1 1 1] Spawn Key
  (if (and (>= (`self.Trigger1_UnlockTriggerAmount`) (`self.Trigger1_MaxTriggerAmount`)) (>= (`self.Trigger2_UnlockTriggerAmount`) (`self.Trigger2_MaxTriggerAmount`)))
    (`/Engine/EditorBlueprintResources/StandardMacros.DoOnce` false
      (:`Completed`
        (`|SpawnActorFromClass` "/Game/Blueprint/BP_Key.BP_Key_C" (`self.KeySpawnTransform`) "Undefined" "MultiplyWithRoot" null null)))))

(event `self.ReceiveBeginPlay`
  ;[1 1 1] Spawns Game UI
  (bind _returnvalue (`|CreateWidget` "/Game/UI/WB_GameUI.WB_GameUI_C" (`GameplayStatics.GetPlayerController` 0)))
  (bind _output_get (set `self.WidgetReference` _returnvalue))
  (`UserWidget.AddToViewport` _output_get 0))

(fn `UserConstructionScript`)