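; BP_KeyGroundTrigger is a puzzle ground trigger that accepts a box of a matching type and counts toward spawning a key.
; BoxInteract passes the box to a check against TriggerType; a match stops the box's Locker physics and makes it immovable.
; On first activation, it hands KeySpawnTransform to YolkoGameMode and increments the unlock amount for its trigger type, guarded by IsTriggered and DoOnce.
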(event `/Game/Blueprint/Interface/BPI_BoxInteract.boxInteract`
  (params (BoxVariable :type "/Game/Blueprint/BP_Box Object Reference"))
  ;[1 1 1] Interface
  (`self.enableKeySpawnTrigger` BoxVariable))

(event `enableKeySpawnTrigger`
  (params (box :type "/Game/Blueprint/BP_Box Object Reference"))
  (bind _gamemode (`self.GameMode`))
  ;[1 1 1] Checks if BoxType is valid
  (bind _output_get (set `self.BoxVariable` box))
  (if (== (`/Game/Blueprint/BP_Box.BoxType` _output_get) (`self.TriggerType`))
    (`PrimitiveComponent.SetSimulatePhysics` (`/Game/Blueprint/BP_Box.Locker` (`self.BoxVariable`)) false)
    (set `/Game/Blueprint/BP_Box.isMovable` false (`self.BoxVariable`))
    (if (not (`self.isTriggered`))
      (set `self.isTriggered` true)
      ;[1 1 1] Spawns Key based on Trigger Type
      (bind _asyolko_game_mode_base (cast `/Game/Blueprint/YolkoGameModeBase` (`GameplayStatics.GetGameMode`)))
      (bind _output_get_2 (set `self.GameMode` _asyolko_game_mode_base))
      (set `/Game/Blueprint/YolkoGameModeBase.KeySpawnTransform` (`self.keySpawnTransform`) _output_get_2)
      (switch `string` (`self.TriggerType`)
        (:`Default`
          (`/Engine/EditorBlueprintResources/StandardMacros.DoOnce` false :!label _label
            (:`Completed`
              (`/Game/Blueprint/YolkoGameModeBase.AddTrigger1UnlockAmount` _gamemode))))
        (:`Trigger2`
          (`/Engine/EditorBlueprintResources/StandardMacros.DoOnce` false
            (:`Completed`
              (`/Game/Blueprint/YolkoGameModeBase.AddTrigger2UnlockAmount` _gamemode))))
        (:`Trigger1`
          (goto _label))))))

(fn `UserConstructionScript`)