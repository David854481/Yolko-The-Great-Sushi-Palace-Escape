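; Actor component that gates a door by spawning a key once both Unnie and Unaggie unlock requirements are met.
; Add and remove events adjust a clamped trigger count for each of the two, capped at its own maximum.
; When KeyCanSpawn is set, each add checks both counts and spawns BP_Key at KeySpawnTransform if both are full.
; No guard in the graph prevents repeat spawns.
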(event `AddUnnieUnlockAmount`
  ;[1 1 1] Unnie Unlock Trigger
  (set `self.Unnie_UnlockTriggerAmount` (`KismetMathLibrary.Clamp` (+ (`self.Unnie_UnlockTriggerAmount`) 1) 0 (`self.Unnie_MaxTriggerAmount`)))
  (if (`self.KeyCanSpawn`)
    (`self.CheckIfDoorUnlockable`)))

(event `RemoveUnnieUnlockAmount`
  ;[1 1 1] Unnie Unlock Trigger
  (set `self.Unnie_UnlockTriggerAmount` (`KismetMathLibrary.Clamp` (- (`self.Unnie_UnlockTriggerAmount`) 1) 0 (`self.Unnie_MaxTriggerAmount`))))

(event `AddUnaggieUnlockAmount`
  ;[1 1 1] Unaggie Unlock Trigger
  (set `self.Unaggie_UnlockTriggerAmount` (`KismetMathLibrary.Clamp` (+ (`self.Unaggie_UnlockTriggerAmount`) 1) 0 (`self.Unaggie_MaxTriggerAmount`)))
  (if (`self.KeyCanSpawn`)
    (`self.CheckIfDoorUnlockable`)))

(event `RemoveUnaggieTriggerAmount`
  ;[1 1 1] Unaggie Unlock Trigger
  (set `self.Unaggie_UnlockTriggerAmount` (`KismetMathLibrary.Clamp` (- (`self.Unaggie_UnlockTriggerAmount`) 1) 0 (`self.Unaggie_MaxTriggerAmount`))))

(event `CheckIfDoorUnlockable`
  ;[1 1 1] Spawn Key
  (if (and (>= (`self.Unaggie_UnlockTriggerAmount`) (`self.Unaggie_MaxTriggerAmount`)) (>= (`self.Unnie_UnlockTriggerAmount`) (`self.Unnie_MaxTriggerAmount`)))
    (`|SpawnActorFromClass` "/Game/Blueprint/BP_Key.BP_Key_C" (`self.KeySpawnTransform`) "Undefined" "MultiplyWithRoot" null null)))