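; Game instance for Yolko that provides shared background music playback and dialogue cutscene triggers.
; PlayMusic starts the BGM cue once as a 2D sound that persists across level transitions, guarded by a playing flag.
; PlayCutscene checks a per-index triggered flag without setting it, then shows the cursor, pauses and opens WB_Dialogue at a given point in UI-only input.
; PlayCutsceneHint does likewise without the flag check or cursor change.
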(event `self.ReceiveInit`)

(fn `Play Cutscene`
  (params (CutsceneIndex :type Integer) (TextLeftParameter :type Integer) (NewIndexParameter :type Integer))
  (bind _returnvalue (`GameplayStatics.GetPlayerController` 0))
  (if (not (`|GetArrayItem` (`self.isCutsceneTriggered`) CutsceneIndex))
    (set `PlayerController.bShowMouseCursor` true _returnvalue)
    (`WidgetBlueprintLibrary.SetInputMode_UIOnlyEx` _returnvalue null)
    (`GameplayStatics.SetGamePaused` true)
    (bind _returnvalue_2 (`|CreateWidget` "/Game/UI/WB_Dialogue.WB_Dialogue_C"))
    (`/Game/UI/WB_Dialogue.Set Dialogue Point` _returnvalue_2 TextLeftParameter NewIndexParameter)
    (`UserWidget.AddToViewport` _returnvalue_2 10)))

(fn `Play Music`
  (if (not (`self.playingMusic`))
    (bind _returnvalue (`GameplayStatics.CreateSound2D` "/Game/Audio/BGM_Cue.BGM_Cue" 0.8 1.0 0.0 "/Game/Audio/YolkoSoundConcurrency.YolkoSoundConcurrency" true))
    (bind _output_get (set `self.Music` _returnvalue))
    (`AudioComponent.Play` _output_get 0.0)
    (set `self.playingMusic` true)))

(fn `PlayCutsceneHint`
  (params (TextLeftParameter :type Integer) (NewIndexParameter :type Integer))
  (`WidgetBlueprintLibrary.SetInputMode_UIOnlyEx` (`GameplayStatics.GetPlayerController` 0) null)
  (`GameplayStatics.SetGamePaused` true)
  (bind _returnvalue (`|CreateWidget` "/Game/UI/WB_Dialogue.WB_Dialogue_C"))
  (`/Game/UI/WB_Dialogue.Set Dialogue Point` _returnvalue TextLeftParameter NewIndexParameter)
  (`UserWidget.AddToViewport` _returnvalue 10))