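; BP_Box is a pushable box that the player moves by contact and that can trigger other actors, noted as key spawning.
; Player overlap on either axis collision turns on Locker physics and plays a drag sound if IsMovable is set, otherwise physics is turned off.
; Its ground trigger sends BoxInteractMessage with itself to any overlapping actor, leaving the response to that actor.
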(event `self.X Axis Collision.OnComponentBeginOverlap`
  (params (OverlappedComponent :type "PrimitiveComponent Object Reference") (OtherActor :type "Actor Object Reference") (OtherComp :type "PrimitiveComponent Object Reference") (OtherBodyIndex :type Integer) (bFromSweep :type Boolean) (SweepResult :type "HitResult Structure (by ref)"))
  ;[1 1 1] Push Box
  (cast `/Game/Blueprint/BP_Player` OtherActor)
  (if (`self.isMovable`) :!label _label
    (`PrimitiveComponent.SetSimulatePhysics` (`self.Locker`) true)
    (`GameplayStatics.PlaySound2D` "/Game/Audio/Object_dragged_FIXED.Object_dragged_FIXED" 0.3 1.0 0.0 null null)
    (else
      (`PrimitiveComponent.SetSimulatePhysics` (`self.Locker`) false))))

(event `self.Y Axis Collision.OnComponentBeginOverlap`
  (params (OverlappedComponent :type "PrimitiveComponent Object Reference") (OtherActor :type "Actor Object Reference") (OtherComp :type "PrimitiveComponent Object Reference") (OtherBodyIndex :type Integer) (bFromSweep :type Boolean) (SweepResult :type "HitResult Structure (by ref)"))
  ;[1 1 1] Push Box
  (cast `/Game/Blueprint/BP_Player` OtherActor)
  (goto _label))

(event `self.Ground Trigger Collision.OnComponentBeginOverlap`
  (params (OverlappedComponent :type "PrimitiveComponent Object Reference") (OtherActor :type "Actor Object Reference") (OtherComp :type "PrimitiveComponent Object Reference") (OtherBodyIndex :type Integer) (bFromSweep :type Boolean) (SweepResult :type "HitResult Structure (by ref)"))
  ;[1 1 1] Trigger Key Spawn
  (message `/Game/Blueprint/Interface/BPI_BoxInteract.boxInteract` OtherActor self))

(fn `UserConstructionScript`)